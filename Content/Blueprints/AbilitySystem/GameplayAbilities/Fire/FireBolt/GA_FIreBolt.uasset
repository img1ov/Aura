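; GA_FireBolt is a gameplay ability that casts a fire bolt projectile toward the cursor target.
; On activation, a TargetDataUnderMouse task supplies the cursor hit location, and the avatar turns to face it through the CombatInterface.
; It plays the cast montage, waits for the montage gameplay event, spawns the projectile at that target, then ends after a short delay.
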(event Ability|EventActivateAbility
  ;[0.15 0.15 0.15 0.5] Active TargetDataUnderMouse task to receive CursorHit data from client
  (bind _datahandle (|TargetDataUnderMouse)
    (:ValidData
      (Variables|Default|SetProjectileTargetLocaton (.Location (Collision|BreakHitResult (Ability|TargetData|GetHitResultfromTargetData _datahandle))))
      (bind _ascombat_interface (Utilities|Casting|CastToCombatInterface (Ability|GetAvatarActorfromActorInfo)))
      (Class|CombatInterface|UpdateFacingTarget _ascombat_interface (Variables|Default|GetProjectileTargetLocaton))
      (|PlayMontageandWaitProxy "None" "/Game/Assets/Characters/Aura/Animations/Abilities/AM_Cast_FireBolt.AM_Cast_FireBolt" 1.0 "None" true 1.0 0.0 false
        (:then
          (Ability|Tasks|WaitGameplayEvent "(TagName=\"Event.Montage.FIreBolt\")" 0
            (:EventReceived
              (Class|AuraProjectileSpell|SpawnProjectile (Variables|Default|GetProjectileTargetLocaton))
              (Utilities|FlowControl|Delay 0.3)
              (Ability|EndAbility))))))))